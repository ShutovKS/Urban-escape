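; BP_MasterItem is an interactable item, apparently a base class, that shows an interact hint to the player.
; Sphere overlap with BP_Character creates a WBP_Interact widget, plays its pop-up, applies an outline overlay material and sets CanPressE.
; Exit reverses these and removes the widget after a short delay.
; CanReceiveTrace toggles the same hint, outline and flag on an existing widget; the interaction itself is not handled here.
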(event OnComponentEndOverlap(Sphere)
  (params (OverlappedComponent :type Primitive%20Component%20Object%20Reference) (OtherActor :type Actor%20Object%20Reference) (OtherComp :type Primitive%20Component%20Object%20Reference) (OtherBodyIndex :type Integer))
  ;[0.15 0.15 0.15 0.5] Trigger Exit
  (Utilities|Casting|CastToBP_Character OtherActor)
  (if (Variables|Default|GetCanInteract)
    (bind _ui_interact (Variables|Default|GetUI%20Interact)
      (:then
        (if (Variables|Default|GetHintVisible)
          (UserInterface|Animation|PlayAnimation _ui_interact (Variables|/Game/_ProjectFiles/Gameplay/UI/WBP_Interact.WBP_Interact_C|GetPopUp _ui_interact) 0.0 1 "Reverse" 1.0 false)
          (Variables|Default|SetHintVisible false)
          (Variables|Default|SetCanPressE false)
          (Rendering|Material|SetOverlayMaterial (Variables|Default|GetStaticMesh) 0 :!class /Script/Engine.MeshComponent)
          (Utilities|FlowControl|Delay 0.15 :!label _label)
          (Widget|RemovefromParent (Variables|Default|GetUI%20Interact))
          (Variables|Default|SetUI%20Interact 0)
          (Rendering|SetVisibility (Variables|Default|GetWidget) false false)))
      (:else
        (goto _label)))))

(event OnComponentBeginOverlap(Sphere)
  (params (OverlappedComponent :type Primitive%20Component%20Object%20Reference) (OtherActor :type Actor%20Object%20Reference) (OtherComp :type Primitive%20Component%20Object%20Reference) (OtherBodyIndex :type Integer) (bFromSweep :type Boolean) (SweepResult :type Hit%20Result%20Structure%20%28by%20ref%29))
  (bind _widget (Variables|Default|GetWidget))
  ;[0.15 0.15 0.15 0.5] Trigger Enter
  (Utilities|Casting|CastToBP_Character OtherActor)
  (if (Variables|Default|GetCanInteract)
    (bind _returnvalue (UserInterface|CreateWidget "/Game/_ProjectFiles/Gameplay/UI/WBP_Interact.WBP_Interact_C"))
    (bind _output_get (Variables|Default|SetUI%20Interact _returnvalue))
    (UserInterface|SetWidget _widget _output_get)
    (Rendering|SetVisibility _widget true false)
    (bind _ui_interact (Variables|Default|GetUI%20Interact)
      (:then
        (if (not (Variables|Default|GetHintVisible))
          (UserInterface|Animation|PlayAnimation _ui_interact (Variables|/Game/_ProjectFiles/Gameplay/UI/WBP_Interact.WBP_Interact_C|GetPopUp _ui_interact) 0.0 1 "Forward" 1.0 false)
          (Variables|Default|SetHintVisible true)
          (Rendering|Material|SetOverlayMaterial (Variables|Default|GetStaticMesh) "/Game/_ProjectFiles/Gameplay/Materials/M_Outline.M_Outline" :!class /Script/Engine.MeshComponent)
          (Variables|Default|SetCanPressE true)))
      (:else))))

(event EventCanReceiveTrace
  (params (Can%20Interact :type Boolean))
  (if (Variables|Default|GetCanInteract)
    (if Can%20Interact
      (bind _ui_interact (Variables|Default|GetUI%20Interact)
        (:then
          (if (not (Variables|Default|GetHintVisible))
            (UserInterface|Animation|PlayAnimation _ui_interact (Variables|/Game/_ProjectFiles/Gameplay/UI/WBP_Interact.WBP_Interact_C|GetPopUp _ui_interact) 0.0 1 "Forward" 1.0 false)
            (Variables|Default|SetHintVisible true)
            (Rendering|Material|SetOverlayMaterial (Variables|Default|GetStaticMesh) "/Game/_ProjectFiles/Gameplay/Materials/M_Outline.M_Outline" :!class /Script/Engine.MeshComponent)
            (Variables|Default|SetCanPressE true)))
        (:else))
      (else
        (bind _ui_interact_2 (Variables|Default|GetUI%20Interact)
          (:then
            (if (Variables|Default|GetHintVisible)
              (UserInterface|Animation|PlayAnimation _ui_interact_2 (Variables|/Game/_ProjectFiles/Gameplay/UI/WBP_Interact.WBP_Interact_C|GetPopUp _ui_interact_2) 0.0 1 "Reverse" 1.0 false)
              (Variables|Default|SetHintVisible false)
              (Rendering|Material|SetOverlayMaterial (Variables|Default|GetStaticMesh) 0 :!class /Script/Engine.MeshComponent)
              (Variables|Default|SetCanPressE false)))
          (:else))))))

(fn ConstructionScript)